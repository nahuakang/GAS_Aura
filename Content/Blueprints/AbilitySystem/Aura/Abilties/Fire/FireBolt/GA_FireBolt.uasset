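; GA_FireBolt is a gameplay ability that casts a fire bolt projectile toward the point under the mouse.
; A TargetDataUnderMouse task supplies the hit location, which the avatar faces through the CombatInterface for motion warping.
; It plays AM_Cast_FireBolt and waits for the montage's Event.Montage.FireBolt gameplay event, sent by an anim notify, to time the projectile spawn before ending the ability.
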(event `self.K2_ActivateAbility`
  ;[1 1 1] Get Projectile Target Location from TargetDataUnderMouse Ability Task
  (bind (_asynctaskproxy _datahandle) (`TargetDataUnderMouse.CreateTargetDataUnderMouse`)
    (:`ValidData`
      (set `self.ProjectileTargetLocation` (`.Location` (`GameplayStatics.BreakHitResult` (`AbilitySystemBlueprintLibrary.GetHitResultFromTargetData` _datahandle))))
      ;[1 1 1] Motion Warping towards ProjectileTargetLocation
      (bind _ascombat_interface (cast `CombatInterface` (`self.GetAvatarActorFromActorInfo`)))
      (`CombatInterface.UpdateFacingTarget` _ascombat_interface (`self.ProjectileTargetLocation`))
      ;[1 1 1] AbilityTask to play montage, wait for montage event from AM_Cast_FireBolt (using custom AN_MontageEvent which overrides ReceivedNotify function to Send Gameplay Event with an EventTag to Actor) and then spawn projectile
      (`AbilityTask_PlayMontageAndWait.CreatePlayMontageAndWaitProxy` "None" "/Game/Assets/Characters/Aura/Animations/Abilities/AM_Cast_FireBolt.AM_Cast_FireBolt"
        (:`then`
          (`AbilityTask_WaitGameplayEvent.WaitGameplayEvent` (struct :`TagName` "Event.Montage.FireBolt") null
            (:`EventReceived`
              (`self.SpawnProjectile` (`self.ProjectileTargetLocation`))
              (`self.K2_EndAbility`))))))))