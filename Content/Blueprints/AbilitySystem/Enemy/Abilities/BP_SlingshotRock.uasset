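; BP_SlingshotRock is the rock actor for an enemy slingshot ability, adding a random tumble to its mesh.
; BeginPlay picks random yaw, pitch and roll rates, each able to spin in either direction.
; Tick applies those rates, scaled by delta seconds, as local rotation on RockMesh for frame-rate-independent spin.
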(event `self.ReceiveBeginPlay`
  (bind _returnvalue (`KismetMathLibrary.RandomFloatInRange` -500.0 500.0))
  ;[1 1 1] Set Yaw Pitch Roll random values
  (set `self.YawRotationRate` _returnvalue)
  (set `self.PitchRotationRate` _returnvalue)
  (set `self.RollRotationRate` _returnvalue))

(event `self.ReceiveTick`
  (params (DeltaSeconds :type "Float (single-precision)"))
  ;[1 1 1] Add random rotation to the rock
  (`SceneComponent.K2_AddLocalRotation` (`self.RockMesh`) (`KismetMathLibrary.MakeRotator` (* DeltaSeconds (`self.RollRotationRate`)) (* DeltaSeconds (`self.PitchRotationRate`)) (* DeltaSeconds (`self.YawRotationRate`))) false false))

(fn `UserConstructionScript`)